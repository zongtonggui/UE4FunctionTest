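; BP_TestController is a test controller for downloading an image and showing it in a UI widget.
; BeginPlay creates MainUI, adds it to the viewport, then loads a texture from a hard-coded disk path into the widget's Image.
; Key 1 calls DownLoad with a fixed image URL.
; Key 2 re-runs the disk load and brush update, reusing the existing widget.
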(event `Key|One`
  (params (Key :type "Key Structure"))
  (:`Pressed`
    (`self.DownLoad` "http://wenwen.soso.com/p/20100214/20100214104541-844772219.jpg")))

(event `self.ReceiveBeginPlay`
  (bind _returnvalue (`|CreateWidget` "/Game/MainUI.MainUI_C"))
  (bind _output_get (set `self.MainUI` _returnvalue))
  (`UserWidget.AddToViewport` _output_get 0)
  (bind _returnvalue_2 (`self.GetTexture2DFromDiskFile` "D:\\Test\\TestC_419\\Saved\\20100214104541-844772219.jpg" (`self.NewVar_0`) :!label _label))
  (`Border.SetBrushFromTexture` (`/Game/MainUI.Image` (`self.MainUI`)) _returnvalue_2))

(event `Key|Two`
  (params (Key :type "Key Structure"))
  (:`Pressed`
    (goto _label)))

(fn `UserConstructionScript`)