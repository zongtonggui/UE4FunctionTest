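; Player controller that displays a texture asset in a UI image through debug key presses.
; On BeginPlay it creates the MainUI widget and adds it to the viewport.
; Key 6 applies the Myobject texture to the widget's Image, or prints an invalid notice when the reference is not valid.
; Key 7 prints the display name of Myobject, which is not assigned in these graphs.
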(event `self.ReceiveBeginPlay`
  (bind _returnvalue (`|CreateWidget` "/Game/MainUI.MainUI_C"))
  (bind _output_get (set `self.MainUI` _returnvalue))
  (`UserWidget.AddToViewport` _output_get 0))

(event `Key|Six`
  (params (Key :type "Key Structure"))
  (bind _myobject (`self.myobject`))
  (:`Pressed`
    (`/Engine/EditorBlueprintResources/StandardMacros.IsValid` _myobject
      (:`Is Valid`
        (`Border.SetBrushFromTexture` (`/Game/MainUI.Image` (`self.MainUI`)) _myobject))
      (:`Is Not Valid`
        (`KismetSystemLibrary.PrintString` "无效")))))

(event `Key|Seven`
  (params (Key :type "Key Structure"))
  (:`Pressed`
    (`KismetSystemLibrary.PrintString` (`KismetSystemLibrary.GetDisplayName` (`self.myobject`)))))

(fn `UserConstructionScript`)