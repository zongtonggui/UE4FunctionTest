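; BP_Controller shows the main menu and provides hotkeys for recording replays.
; On BeginPlay it adds WID_MainMenu to the viewport and shows the mouse cursor for player 0.
; PageUp and PageDown start and stop recording through BP_MyGameInstance, printing a Chinese status message.
; Replay names are built from the current date and time, and recording requests the InMemoryNetworkReplayStreaming streamer instead of the default.
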(event `self.ReceiveBeginPlay`
  (bind _returnvalue (`GameplayStatics.GetPlayerController` 0))
  (bind _returnvalue_2 (`|CreateWidget` "/Game/WID_MainMenu.WID_MainMenu_C" _returnvalue))
  (`/Engine/EditorBlueprintResources/StandardMacros.IsValid` _returnvalue_2
    (:`Is Valid`
      (`UserWidget.AddToViewport` _returnvalue_2 0)
      (set `PlayerController.bShowMouseCursor` true _returnvalue))))

(event `Key|PageUp`
  (params (Key :type "Key Structure"))
  (bind (_year _month _day _hour _minute _second) (`KismetMathLibrary.BreakDateTime` (`KismetMathLibrary.Now`)))
  (:`Pressed`
    (bind _asbp_my_game_instance (cast `/Game/BP_MyGameInstance` (`GameplayStatics.GetGameInstance`)))
    (`MyGameInstance.StartRecordingReplayFromBP` _asbp_my_game_instance (`KismetStringLibrary.Concat_StrStr` "Replay_" (`KismetStringLibrary.Conv_IntToString` _year) "_" (`KismetStringLibrary.Conv_IntToString` _month) "_" (`KismetStringLibrary.Conv_IntToString` _day) "_" (`KismetStringLibrary.Conv_IntToString` _hour) "_" (`KismetStringLibrary.Conv_IntToString` _minute) "_" (`KismetStringLibrary.Conv_IntToString` _second)) "Test" (`|MakeArray` "ReplayStreamerOverride = InMemoryNetworkReplayStreaming"))
    (`KismetSystemLibrary.PrintString` "开始录制")))

(event `Key|PageDown`
  (params (Key :type "Key Structure"))
  (:`Pressed`
    (bind _asbp_my_game_instance (cast `/Game/BP_MyGameInstance` (`GameplayStatics.GetGameInstance`)))
    (`MyGameInstance.StopRecordingReplayFromBP` _asbp_my_game_instance)
    (`KismetSystemLibrary.PrintString` "结束录制")))

(fn `UserConstructionScript`)